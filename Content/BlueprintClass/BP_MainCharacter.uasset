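; Player character for a flying game that moves forward automatically along control yaw, steered sideways and vertically by mouse axes.
; The Impulso action quadruples fly speed on press but only halves it on release, replaying a timeline meant to ease camera FOV between wide values.
; Death spawns an explosion, then pauses and shows the Muerte widget after a delay; Victory plays a sound, pauses and shows its widget.
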(event Custom|Death
  (bind _returnvalue (Game|GetPlayerController 0))
  (Effects|SpawnEmitteratLocation "/Game/StarterContent/Particles/P_Explosion.P_Explosion" (Transformation|GetActorLocation))
  (Components|Activation|Deactivate (Variables|Character|GetCharacterMovement))
  (Utilities|FlowControl|Delay 0.7)
  (Game|SetGamePaused true)
  (bind _returnvalue_2 (UserInterface|CreateWidget "/Game/Widgets/Muerte.Muerte_C" (Game|GetPlayerController 0)))
  (UserInterface|Viewport|AddtoPlayerScreen _returnvalue_2)
  (Input|SetInputModeUIOnly _returnvalue _returnvalue_2 "DoNotLock" false)
  (Variables|/Script/Engine.PlayerController|SetbShowMouseCursor _returnvalue true))

(event Custom|Victory
  (Audio|PlaySound2D "/Game/Sounds/efecto_de_sonido_victoria_happy_wheels__1_.efecto_de_sonido_victoria_happy_wheels__1_" 1.0 1.0 0.0 0 0)
  (Components|Activation|Deactivate (Variables|Character|GetCharacterMovement))
  (Game|SetGamePaused true)
  (bind _returnvalue (UserInterface|CreateWidget "/Game/Widgets/Victory.Victory_C"))
  (UserInterface|Viewport|AddtoPlayerScreen _returnvalue))

(event EventBeginPlay
  (Pawn|Components|CharacterMovement|SetMovementMode (Variables|Character|GetCharacterMovement) "MOVE_Flying" 0))

(event EventTick
  (params (DeltaSeconds :type Float%20%28single-precision%29))
  (Pawn|Input|AddMovementInput (Math|Vector|GetForwardVector (Math|Rotator|MakeRotator 0.0 0.0 (.Yaw (Math|Rotator|BreakRotator (Pawn|GetControlRotation :!class /Script/Engine.Pawn))))) (Variables|Default|GetMovement) false))

(event Input|ActionEvents|InputActionImpulso
  (params (Key :type Key%20Structure :default "None"))
  (bind _charactermovement (Variables|Character|GetCharacterMovement))
  (:Pressed
    (Variables|/Script/Engine.CharacterMovementComponent|SetMaxFlySpeed _charactermovement (* (Variables|/Script/Engine.CharacterMovementComponent|GetMaxFlySpeed _charactermovement) 4.0))
    (Variables|Default|SetNewFieldOfView 1.4e+02)
    (Components|Timeline|PlayfromStart (Variables|Default|GetFieldOfView) :!label _label))
  (:Released
    (Variables|/Script/Engine.CharacterMovementComponent|SetMaxFlySpeed _charactermovement (/ (Variables|/Script/Engine.CharacterMovementComponent|GetMaxFlySpeed _charactermovement) 2.0))
    (Variables|Default|SetNewFieldOfView 1.2e+02)
    (goto _label)))

(event Input|AxisEvents|InputAxisLeftRightMouse
  (params (AxisValue :type Float%20%28single-precision%29))
  (Pawn|Input|AddMovementInput (Math|Vector|GetRightVector (Math|Rotator|MakeRotator 0.0 0.0 (.Yaw (Math|Rotator|BreakRotator (Pawn|GetControlRotation :!class /Script/Engine.Pawn))))) AxisValue false)
  (if (>= AxisValue 1.0)
    (Variables|Default|SetDirection 9e+01)
    (elif (<= AxisValue -1.0)
      (Variables|Default|SetDirection -9e+01)
      (else
        (Variables|Default|SetDirection 0.0)))))

(event Input|AxisEvents|InputAxisMoveRight
  (params (AxisValue :type Float%20%28single-precision%29)))

(event Input|AxisEvents|InputAxisMoveUp
  (params (AxisValue :type Float%20%28single-precision%29)))

(event Input|AxisEvents|InputAxisUpDownMouse
  (params (AxisValue :type Float%20%28single-precision%29))
  (Pawn|Input|AddMovementInput (Math|Vector|GetUpVector (Math|Rotator|MakeRotator 0.0 0.0 (.Yaw (Math|Rotator|BreakRotator (Pawn|GetControlRotation :!class /Script/Engine.Pawn))))) AxisValue false))

(fn ConstructionScript)